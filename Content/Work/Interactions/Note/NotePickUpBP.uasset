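; Collectible note pickup actor that displays a note widget and counts toward the notes collected in MyGameInstance.
; Its mesh material follows the NoteCard index, which overlap copies to the first-person character while enabling input and showing a CameraHUD prompt.
; An Interact FlipFlop opens the note and increments the count, then closes it.
; Closing or ending overlap, even unread, clears the prompt and destroys the actor.
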(event `self.ReceiveBeginPlay`
  (`PrimitiveComponent.SetMaterial` (`self.StaticMesh`) 0 (`|GetArrayItem` (`self.MaterialIndex`) (`self.NoteCard`))))

(event `EnhancedInput|/Game/Work/Player/FirstPerson/Input/Actions/IA_Interact`
  (params (ActionValue :type Boolean) (ElapsedSeconds :type "Float (double-precision)") (TriggeredSeconds :type "Float (double-precision)") (InputAction :type "InputAction Object Reference" :default "/Game/Work/Player/FirstPerson/Input/Actions/IA_Interact.IA_Interact"))
  (:`Triggered`
    (`/Engine/EditorBlueprintResources/StandardMacros.FlipFlop`
      (:`A`
        (bind _returnvalue (`|CreateWidget` "/Game/Work/UserInterface/Notes/NotePickUpWBP.NotePickUpWBP_C"))
        (`UserWidget.AddToViewport` _returnvalue 0)
        (bind _asmy_game_instance (cast `/Game/Work/Instance/MyGameInstance` (`GameplayStatics.GetGameInstance`)))
        (set `/Game/Work/Instance/MyGameInstance.GI_NotesColleceted` (+ (`/Game/Work/Instance/MyGameInstance.GI_NotesColleceted` _asmy_game_instance) 1) _asmy_game_instance))
      (:`B`
        (`Widget.RemoveFromParent` _returnvalue :!label _label)
        (bind _foundwidgets (`WidgetBlueprintLibrary.GetAllWidgetsOfClass` "/Game/Work/UserInterface/Player/CameraHUD.CameraHUD_C"))
        (`TextBlock.SetText` (`/Game/Work/UserInterface/Player/CameraHUD.TextBlock_39` (`|GetArrayItem` _foundwidgets)) "")
        (`self.K2_DestroyActor`)))))

(event `self.ReceiveActorEndOverlap`
  (params (OtherActor :type "Actor Object Reference"))
  (`self.DisableInput` (`GameplayStatics.GetPlayerController` 0))
  (goto _label))

(event `self.ReceiveActorBeginOverlap`
  (params (OtherActor :type "Actor Object Reference"))
  (`self.EnableInput` (`GameplayStatics.GetPlayerController` 0))
  (bind _asbp_first_person_character (cast `/Game/Work/Player/FirstPerson/Blueprints/BP_FirstPersonCharacter` (`GameplayStatics.GetPlayerCharacter` 0)))
  (set `/Game/Work/Player/FirstPerson/Blueprints/BP_FirstPersonCharacter.NoteCardIndex` (`self.NoteCard`) _asbp_first_person_character)
  (bind _foundwidgets (`WidgetBlueprintLibrary.GetAllWidgetsOfClass` "/Game/Work/UserInterface/Player/CameraHUD.CameraHUD_C"))
  (`TextBlock.SetText` (`/Game/Work/UserInterface/Player/CameraHUD.TextBlock_39` (`|GetArrayItem` _foundwidgets)) "Press \"E\" To Interact With Note"))

(fn `UserConstructionScript`)