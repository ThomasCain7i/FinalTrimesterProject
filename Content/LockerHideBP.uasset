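; Hideable locker actor that lets the first-person player hide inside by pressing Interact while overlapping it.
; Overlap shows a CameraHUD prompt and enables actor input through a Gate, which end overlap closes and a post-toggle delay reopens.
; Interacting toggles the player's visibility and collision, blends the camera between player and locker, and plays a timeline that swings the door.
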(event `EnhancedInput|/Game/FirstPerson/Input/Actions/IA_Interact`
  (params (ActionValue :type Boolean) (ElapsedSeconds :type "Float (double-precision)") (TriggeredSeconds :type "Float (double-precision)") (InputAction :type "InputAction Object Reference" :default "/Game/FirstPerson/Input/Actions/IA_Interact.IA_Interact"))
  ;[1 1 1] Gein In & Out Of Locker
  (:`Triggered`
    (`/Engine/EditorBlueprintResources/StandardMacros.Gate` true :!label _label
      (:`Exit`
        (`|ExecutionSequence`
          (:`then_0`
            (`self.ToggleHide`)
            (`KismetSystemLibrary.Delay` 0.8)
            (`self.EnableInput` (`GameplayStatics.GetPlayerController` 0) :!label _label_2)
            (goto _label :!via `Open`))
          (:`then_1`
            (bind (_direction _door_track) (`Timeline|Open/Close Door Timeline` :!via `PlayFromStart`)
              (:`Update`
                (`SceneComponent.K2_SetRelativeRotation` (`self.Locker Door`) (`KismetMathLibrary.MakeRotator` 90.0 0.0 (`KismetMathLibrary.Lerp` (`self.CloseAngle`) (`self.Open Angle`) _door_track)) false false)))))))))

(event `self.ReceiveActorBeginOverlap`
  (params (OtherActor :type "Actor Object Reference"))
  ;[1 1 1] Gein In & Out Of Locker
  (bind _asbp_first_person_character (cast `/Game/FirstPerson/Blueprints/BP_FirstPersonCharacter` OtherActor))
  (set `self.Player REF` _asbp_first_person_character)
  (bind _foundwidgets (`WidgetBlueprintLibrary.GetAllWidgetsOfClass` "/Game/UI/CameraHUD.CameraHUD_C"))
  (`TextBlock.SetText` (`/Game/UI/CameraHUD.TextBlock_39` (`|GetArrayItem` _foundwidgets)) "Press \"E\" To Hide")
  (goto _label_2))

(event `self.ReceiveActorEndOverlap`
  (params (OtherActor :type "Actor Object Reference"))
  ;[1 1 1] Gein In & Out Of Locker
  (cast `/Game/FirstPerson/Blueprints/BP_FirstPersonCharacter` OtherActor)
  (`self.DisableInput` (`GameplayStatics.GetPlayerController` 0))
  (bind _foundwidgets (`WidgetBlueprintLibrary.GetAllWidgetsOfClass` "/Game/UI/CameraHUD.CameraHUD_C"))
  (`TextBlock.SetText` (`/Game/UI/CameraHUD.TextBlock_39` (`|GetArrayItem` _foundwidgets)) "")
  (`self.EnableInput` null)
  (goto _label :!via `Close`))

(fn `ToggleHide`
  (bind _returnvalue (`GameplayStatics.GetPlayerController` 0))
  (bind _player_ref (`self.Player REF`))
  (if (`self.IsHiding?`)
    (set `self.IsHiding?` false)
    (`self.SetActorHiddenInGame` _player_ref false)
    (`self.SetActorEnableCollision` _player_ref true)
    (`PlayerController.SetViewTargetWithBlend` _returnvalue _player_ref 0.8 "VTBlend_Linear" 0.0 false)
    (else
      (set `self.IsHiding?` true)
      (`self.SetActorHiddenInGame` _player_ref true)
      (`self.SetActorEnableCollision` _player_ref false)
      (`PlayerController.SetViewTargetWithBlend` _returnvalue self 0.8 "VTBlend_Linear" 0.0 false))))

(fn `UserConstructionScript`)