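; Interactable door actor that swings open and closed on its yaw when Interact is called.
; The OpenDoor timeline plays or reverses based on IsOpen, with play rate set from separate open and close times, lerping rotation up to DoorOpensDegree.
; IsOpen flips when the timeline finishes.
; Overlapping the actor shows a "Press E" prompt on the CameraHUD widget, cleared when overlap ends.
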(event `/Game/Interactions/Interact_Interface.Interact`
  (bind _opendoor (`self.OpenDoor`))
  (if (not (`self.IsOpen?`))
    (`TimelineComponent.SetPlayRate` _opendoor (/ 1.0 (`self.TimeToOpen`)))
    (bind (_direction _opendoor_2) (`Timeline|OpenDoor` :!label _label)
      (:`Update`
        (`SceneComponent.K2_SetRelativeRotation` (`self.Door`) (`KismetMathLibrary.MakeRotator` 0.0 0.0 (`KismetMathLibrary.Lerp` 0.0 (`self.Door Opens Degree`) _opendoor_2)) false false))
      (:`Finished`
        (set `self.IsOpen?` (not (`self.IsOpen?`)))))
    (else
      (`TimelineComponent.SetPlayRate` _opendoor (/ 1.0 (`self.TimeToClose`)))
      (goto _label :!via `Reverse`))))

(event `self.ReceiveActorBeginOverlap`
  (params (OtherActor :type "Actor Object Reference"))
  (bind _foundwidgets (`WidgetBlueprintLibrary.GetAllWidgetsOfClass` "/Game/UI/CameraHUD.CameraHUD_C"))
  (`TextBlock.SetText` (`/Game/UI/CameraHUD.TextBlock_39` (`|GetArrayItem` _foundwidgets)) "Press \"E\" To Interact"))

(event `self.ReceiveActorEndOverlap`
  (params (OtherActor :type "Actor Object Reference"))
  (bind _foundwidgets (`WidgetBlueprintLibrary.GetAllWidgetsOfClass` "/Game/UI/CameraHUD.CameraHUD_C"))
  (`TextBlock.SetText` (`/Game/UI/CameraHUD.TextBlock_39` (`|GetArrayItem` _foundwidgets)) ""))

(fn `UserConstructionScript`)