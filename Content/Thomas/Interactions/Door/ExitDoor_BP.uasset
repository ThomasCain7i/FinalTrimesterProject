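; ExitDoor_BP is a double exit door that opens only when the player has the key and the power is on.
; Interact plays a sound and runs a timeline that swings both leaves open once by lerping their yaw, or shows "LOCKED" on the CameraHUD.
; Overlapping the actor with the Player tag shows an interact prompt for keyboard or controller, chosen from the game instance, and clears it on exit.
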(event `self.ReceiveBeginPlay`
  (bind _asmy_game_instance (cast `/Game/Thomas/Instance/MyGameInstance` (`GameplayStatics.GetGameInstance`)))
  (set `self.Game Instance REF` _asmy_game_instance)
  (bind _asbp_first_person_character (cast `/Game/Thomas/Player/FirstPerson/Blueprints/BP_FirstPersonCharacter` (`GameplayStatics.GetPlayerCharacter` 0)))
  (set `self.Player REF` _asbp_first_person_character))

(event `self.Interact`
  (bind _player_ref (`self.Player REF`))
  (if (and (`/Game/Thomas/Player/FirstPerson/Blueprints/BP_FirstPersonCharacter.HasKey?` _player_ref) (`/Game/Thomas/Player/FirstPerson/Blueprints/BP_FirstPersonCharacter.PowerOn?` _player_ref))
    (if (not (`self.IsOpen?`))
      (`TimelineComponent.SetPlayRate` (`self.OpenDoor`) (/ 1.0 (`self.TimeToOpen`)))
      (`GameplayStatics.PlaySoundAtLocation` "/Game/Audio/WoodDoor/OpenWoodDoorCue.OpenWoodDoorCue" (0.0 0.0 0.0) (struct) 1.0 0.5 0.0 null null null null)
      (bind (_direction _exitdoortrack) (`Timeline|OpenDoor`)
        (:`Update`
          (`SceneComponent.K2_SetRelativeRotation` (`self.LeftDoor`) (`KismetMathLibrary.MakeRotator` 0.0 0.0 (`KismetMathLibrary.Lerp` 0.0 (`self.Left Door Opens Degree`) _exitdoortrack)) false false)
          (`SceneComponent.K2_SetRelativeRotation` (`self.RightDoor`) (`KismetMathLibrary.MakeRotator` 0.0 0.0 (`KismetMathLibrary.Lerp` 180.0 (`self.Right Door Opens Degree_0`) _exitdoortrack)) false false)
          (set `self.IsOpen?` true))))
    (else
      (bind _foundwidgets (`WidgetBlueprintLibrary.GetAllWidgetsOfClass` "/Game/Thomas/UserInterface/HUD/CameraHUD.CameraHUD_C"))
      (`TextBlock.SetText` (`/Game/Thomas/UserInterface/HUD/CameraHUD.InteractText` (`|GetArrayItem` _foundwidgets)) "LOCKED"))))

(event `self.ReceiveActorBeginOverlap`
  (params (OtherActor :type "Actor Object Reference"))
  (if (`self.ActorHasTag` OtherActor "Player")
    (bind _foundwidgets (`WidgetBlueprintLibrary.GetAllWidgetsOfClass` "/Game/Thomas/UserInterface/HUD/CameraHUD.CameraHUD_C"))
    (if (`/Game/Thomas/Instance/MyGameInstance.GI_Controller?` (`self.Game Instance REF`))
      (bind _interacttext (`/Game/Thomas/UserInterface/HUD/CameraHUD.InteractText` (`|GetArrayItem` _foundwidgets)))
      (`TextBlock.SetText` _interacttext "Press \"X\" To Interact")
      (else
        (`TextBlock.SetText` _interacttext "Press \"E\" To Interact")))))

(event `self.ReceiveActorEndOverlap`
  (params (OtherActor :type "Actor Object Reference"))
  (if (`self.ActorHasTag` OtherActor "Player")
    (bind _foundwidgets (`WidgetBlueprintLibrary.GetAllWidgetsOfClass` "/Game/Thomas/UserInterface/HUD/CameraHUD.CameraHUD_C"))
    (`TextBlock.SetText` (`/Game/Thomas/UserInterface/HUD/CameraHUD.InteractText` (`|GetArrayItem` _foundwidgets)) "")))

(fn `UserConstructionScript`)