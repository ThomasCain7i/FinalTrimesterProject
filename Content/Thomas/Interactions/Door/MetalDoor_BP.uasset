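; MetalDoor_BP is an interactable swinging door that opens and closes on Interact.
; An OpenDoor timeline lerps the door's yaw, with play rate set from open/close times, wood-door cues played at world origin, and IsOpen flipped on finish.
; Player overlap shows a keyboard or controller prompt on CameraHUD, chosen via the game instance, and clears it on exit.
; Any non-player overlap plays the opening timeline directly if IsOpen is false, without sound.
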(event `self.ReceiveBeginPlay`
  (bind _asmy_game_instance (cast `/Game/Thomas/Instance/MyGameInstance` (`GameplayStatics.GetGameInstance`)))
  (set `self.Game Instance REF` _asmy_game_instance))

(event `self.Interact`
  (bind _opendoor (`self.OpenDoor`))
  (if (not (`self.IsOpen?`))
    (`TimelineComponent.SetPlayRate` _opendoor (/ 1.0 (`self.TimeToOpen`)))
    (`GameplayStatics.PlaySoundAtLocation` "/Game/Audio/WoodDoor/OpenWoodDoorCue.OpenWoodDoorCue" (0.0 0.0 0.0) (struct) 1.0 1.0 0.0 null null null null)
    (bind (_direction _opendoor_2) (`Timeline|OpenDoor` :!label _label)
      (:`Update`
        (`SceneComponent.K2_SetRelativeRotation` (`self.Door`) (`KismetMathLibrary.MakeRotator` 0.0 0.0 (`KismetMathLibrary.Lerp` 0.0 (`self.Door Opens Degree`) _opendoor_2)) false false))
      (:`Finished`
        (set `self.IsOpen?` (not (`self.IsOpen?`)))))
    (else
      (`TimelineComponent.SetPlayRate` _opendoor (/ 1.0 (`self.TimeToClose`)))
      (`GameplayStatics.PlaySoundAtLocation` "/Game/Audio/WoodDoor/CloseWoodDoorCue.CloseWoodDoorCue" (0.0 0.0 0.0) (struct) 1.0 1.0 0.0 null null null null)
      (goto _label :!via `Reverse`))))

(event `self.ReceiveActorBeginOverlap`
  (params (OtherActor :type "Actor Object Reference"))
  (if (`self.ActorHasTag` OtherActor "Player")
    (bind _foundwidgets (`WidgetBlueprintLibrary.GetAllWidgetsOfClass` "/Game/Thomas/UserInterface/Player/CameraHUD.CameraHUD_C"))
    (if (`/Game/Thomas/Instance/MyGameInstance.GI_Controller?` (`self.Game Instance REF`))
      (bind _interacttext (`/Game/Thomas/UserInterface/Player/CameraHUD.InteractText` (`|GetArrayItem` _foundwidgets)))
      (`TextBlock.SetText` _interacttext "Press \"X\" To Interact")
      (else
        (`TextBlock.SetText` _interacttext "Press \"E\" To Interact")))
    (elif (not (`self.IsOpen?`))
      (goto _label))))

(event `self.ReceiveActorEndOverlap`
  (params (OtherActor :type "Actor Object Reference"))
  (if (`self.ActorHasTag` OtherActor "Player")
    (bind _foundwidgets (`WidgetBlueprintLibrary.GetAllWidgetsOfClass` "/Game/Thomas/UserInterface/Player/CameraHUD.CameraHUD_C"))
    (`TextBlock.SetText` (`/Game/Thomas/UserInterface/Player/CameraHUD.InteractText` (`|GetArrayItem` _foundwidgets)) "")))

(fn `UserConstructionScript`)