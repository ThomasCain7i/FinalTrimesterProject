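; Locked door that swings open on interaction once the player character has a key, otherwise showing "LOCKED" on the CameraHUD.
; A timeline lerps the door's yaw and flips IsOpen on finish; the reverse branch is unreachable behind a repeated IsOpen check.
; Player overlap shows or clears a keyboard or controller prompt based on the game instance.
; Non-player overlaps play the opening timeline without a key check.
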(event `self.ReceiveBeginPlay`
  (bind _asbp_first_person_character (cast `/Game/Thomas/Player/FirstPerson/Blueprints/BP_FirstPersonCharacter` (`GameplayStatics.GetPlayerCharacter` 0)))
  (set `self.Player REF` _asbp_first_person_character)
  (bind _asmy_game_instance (cast `/Game/Thomas/Instance/MyGameInstance` (`GameplayStatics.GetGameInstance`)))
  (set `self.Game Instance REF` _asmy_game_instance))

(event `self.Interact`
  (bind _opendoor (`self.OpenDoor`))
  (if (`self.IsOpen?`)
    _
    (elif (`/Game/Thomas/Player/FirstPerson/Blueprints/BP_FirstPersonCharacter.HasKey?` (`self.Player REF`))
      (if (not (`self.IsOpen?`))
        (`TimelineComponent.SetPlayRate` _opendoor (/ 1.0 (`self.TimeToOpen`)))
        (bind (_direction _opendoor_2) (`Timeline|OpenDoor` :!label _label)
          (:`Update`
            (`SceneComponent.K2_SetRelativeRotation` (`self.Door`) (`KismetMathLibrary.MakeRotator` 90.0 0.0 (`KismetMathLibrary.Lerp` 0.0 (`self.Door Opens Degree`) _opendoor_2)) false false))
          (:`Finished`
            (set `self.IsOpen?` (not (`self.IsOpen?`)))))
        (else
          (`TimelineComponent.SetPlayRate` _opendoor (/ 1.0 (`self.TimeToClose`)))
          (goto _label :!via `Reverse`)))
      (else
        (bind _foundwidgets (`WidgetBlueprintLibrary.GetAllWidgetsOfClass` "/Game/Thomas/UserInterface/Player/CameraHUD.CameraHUD_C"))
        (`TextBlock.SetText` (`/Game/Thomas/UserInterface/Player/CameraHUD.InteractText` (`|GetArrayItem` _foundwidgets)) "LOCKED")))))

(event `self.ReceiveActorBeginOverlap`
  (params (OtherActor :type "Actor Object Reference"))
  (if (`self.ActorHasTag` OtherActor "Player")
    (bind _foundwidgets (`WidgetBlueprintLibrary.GetAllWidgetsOfClass` "/Game/Thomas/UserInterface/Player/CameraHUD.CameraHUD_C"))
    (if (`/Game/Thomas/Instance/MyGameInstance.GI_Controller?` (`self.Game Instance REF`))
      (bind _interacttext (`/Game/Thomas/UserInterface/Player/CameraHUD.InteractText` (`|GetArrayItem` _foundwidgets)))
      (`TextBlock.SetText` _interacttext "Press \"X\" To Interact")
      (else
        (`TextBlock.SetText` _interacttext "Press \"E\" To Interact")))
    (elif (not (`self.IsOpen?`))
      (goto _label))))

(event `self.ReceiveActorEndOverlap`
  (params (OtherActor :type "Actor Object Reference"))
  (if (`self.ActorHasTag` OtherActor "Player")
    (bind _foundwidgets (`WidgetBlueprintLibrary.GetAllWidgetsOfClass` "/Game/Thomas/UserInterface/Player/CameraHUD.CameraHUD_C"))
    (`TextBlock.SetText` (`/Game/Thomas/UserInterface/Player/CameraHUD.InteractText` (`|GetArrayItem` _foundwidgets)) "")))

(fn `UserConstructionScript`)