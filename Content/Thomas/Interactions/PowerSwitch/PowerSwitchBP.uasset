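; PowerSwitchBP is an interactable wall switch that turns on power by setting the PowerOn flag on the player's BP_FirstPersonCharacter.
; Overlap by a Player-tagged actor toggles input on the switch and shows or clears its prompt in the CameraHUD widget.
; IA_Interact works only while power is off, then plays the PowerSwitchDown timeline to set Box's yaw, though the Lerp alpha is fixed at zero.
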(event `self.ReceiveBeginPlay`
  (bind _asbp_first_person_character (cast `/Game/Thomas/Player/FirstPerson/Blueprints/BP_FirstPersonCharacter` (`GameplayStatics.GetPlayerCharacter` 0)))
  (set `self.Player REF` _asbp_first_person_character))

(event `EnhancedInput|/Game/Thomas/Player/FirstPerson/Input/Actions/IA_Interact`
  (params (ActionValue :type Boolean) (ElapsedSeconds :type "Float (double-precision)") (TriggeredSeconds :type "Float (double-precision)") (InputAction :type "InputAction Object Reference" :default "/Game/Thomas/Player/FirstPerson/Input/Actions/IA_Interact.IA_Interact"))
  (bind _player_ref (`self.Player REF`))
  (:`Triggered`
    (if (not (`/Game/Thomas/Player/FirstPerson/Blueprints/BP_FirstPersonCharacter.PowerOn?` _player_ref))
      (set `/Game/Thomas/Player/FirstPerson/Blueprints/BP_FirstPersonCharacter.PowerOn?` true _player_ref)
      (`Timeline|PowerSwitchDown`
        (:`Update`
          (`SceneComponent.K2_SetRelativeRotation` (`self.Box`) (`KismetMathLibrary.MakeRotator` 0.0 0.0 (`KismetMathLibrary.Lerp` 0.0 (`self.PowerSwitchDegrees`))) false false))))))

(event `self.ReceiveActorEndOverlap`
  (params (OtherActor :type "Actor Object Reference"))
  (if (`self.ActorHasTag` OtherActor "Player")
    (`self.DisableInput` (`GameplayStatics.GetPlayerController` 0))
    (bind _foundwidgets (`WidgetBlueprintLibrary.GetAllWidgetsOfClass` "/Game/Thomas/UserInterface/Player/CameraHUD.CameraHUD_C"))
    (`TextBlock.SetText` (`/Game/Thomas/UserInterface/Player/CameraHUD.InteractText` (`|GetArrayItem` _foundwidgets)) "")))

(event `self.ReceiveActorBeginOverlap`
  (params (OtherActor :type "Actor Object Reference"))
  (if (`self.ActorHasTag` OtherActor "Player")
    (`self.EnableInput` (`GameplayStatics.GetPlayerController` 0))
    (bind _foundwidgets (`WidgetBlueprintLibrary.GetAllWidgetsOfClass` "/Game/Thomas/UserInterface/Player/CameraHUD.CameraHUD_C"))
    (`TextBlock.SetText` (`/Game/Thomas/UserInterface/Player/CameraHUD.InteractText` (`|GetArrayItem` _foundwidgets)) (`self.PowerSwitchText`))))

(fn `UserConstructionScript`)